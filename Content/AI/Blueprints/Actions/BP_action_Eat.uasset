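; AI action Blueprint that sends its pawn to the closest food place to eat.
; Task scans all BP_Place_Food actors for the nearest, moves the pawn there with AIMoveTo, then on success sets its yaw and sends StartEatingMessage.
; The yaw look-at uses the pawn's location as both start and target, so it does not face the food.
; Stop sends StopEatingMessage before running the parent stop logic.
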(event `self.Task`
  (bind _pawn (`self.Pawn`))
  (bind (_returnvalue_roll _returnvalue_pitch _returnvalue_yaw) (`KismetMathLibrary.BreakRotator` (`KismetMathLibrary.FindLookAtRotation` (`self.K2_GetActorLocation` (`self.Pawn`)) (`self.K2_GetActorLocation` _pawn))))
  (`parent.Task`)
  (bind _food (`self.GetNearestFood`))
  (`/Engine/EditorBlueprintResources/StandardMacros.IsValid` _food
    (:`Is Valid`
      (`|AIMoveTo` _pawn (`/Game/AI/Blueprints/Places/BP_Place.GetLocation` _food) null (`self.Acceptance Radius`)
        (:`OnSuccess`
          (`self.K2_SetActorRotation` (`self.Pawn`) (`KismetMathLibrary.MakeRotator` 0.0 0.0 _returnvalue_yaw) false)
          (message `/Game/AI/Blueprints/Interface/BPI_Eating.StartEating` (`self.Pawn`)))))))

(event `self.Stop`
  (message `/Game/AI/Blueprints/Interface/BPI_Eating.StopEating` (`self.Pawn`))
  (`parent.Stop`))

(fn `GetNearestFood`
  (returns (Food :type "/Game/AI/Blueprints/Places/BP_Place_Food Object Reference"))
  (bind _outactors (`GameplayStatics.GetAllActorsOfClass` "/Game/AI/Blueprints/Places/BP_Place_Food.BP_Place_Food_C"))
  (set `self.L_NearestFood` (`|GetArrayItem` _outactors))
  (for _array_element _outactors
    (if (< (`self.GetDistanceTo` _array_element (`self.Pawn`)) (`self.GetDistanceTo` (`self.L_NearestFood`) (`self.Pawn`)))
      (set `self.L_NearestFood` _array_element)))
  (return (`self.L_NearestFood`)))

(fn `UserConstructionScript`
  (`parent.UserConstructionScript`))