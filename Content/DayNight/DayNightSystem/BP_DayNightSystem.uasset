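; Day-night system Blueprint that keeps game time as a running count of seconds, seeded from Day, Hour, Minute and Second in the construction script.
; BeginPlay starts a looping timer at an interval of one over Speed, clamped to a minimum.
; ChangeTime advances Time by Speed times that interval, and GetHour and GetDay derive fractional values from it.
; Tick prints the raw Time for debugging.
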(event `self.ReceiveBeginPlay`
  (`KismetSystemLibrary.K2_SetTimerDelegate` (`|CreateDelegate` :!event `ChangeTime`) (`self.GetTimerRate`) true))

(event `self.ReceiveTick`
  (params (DeltaSeconds :type "Float (single-precision)"))
  (`KismetSystemLibrary.PrintString` (`KismetStringLibrary.Conv_DoubleToString` (`self.Time`)) true true (struct :`G` 0.66 :`B` 1.0 :`A` 1.0) 0.0))

(fn `ChangeTime`
  (set `self.Time` (+ (`self.Time`) (* (`self.Speed`) (`self.GetTimerRate`)))))

(fn `GetDay`
  (returns (Days :type "Float (double-precision)"))
  (return (/ (`self.Time`) 86400.0)))

(fn `GetHour`
  (returns (Hours :type "Float (double-precision)"))
  (return (/ (mod (`self.Time`) 86400.0) 3600.0)))

(fn `GetTimerRate`
  (returns (TimerRate :type "Float (double-precision)"))
  (return (`KismetMathLibrary.FMax` (/ 1.0 (`self.Speed`)) 0.01)))

(fn `UserConstructionScript`
  (set `self.Time` (`KismetMathLibrary.Conv_IntToDouble` (+ (* (`self.Day`) 86400) (* (`self.Hour`) 3600) (* (`self.Minute`) 60) (`self.Second`)))))