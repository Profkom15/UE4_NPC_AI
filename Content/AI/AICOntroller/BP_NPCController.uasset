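; BP_NPCController is an AI controller that runs an NPC's daily schedule against the BP_DayNightSystem clock.
; On possess it starts a looping timer at the day/night timer rate to re-check the current action.
; GetaAction picks an action class from the pawn's hour-keyed schedule, assuming ascending keys and wrapping overnight to the last entry.
; When that class changes, it stops the old action and spawns the new action actor; Tick prints debug info.
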(event `self.ReceiveTick`
  (params (DeltaSeconds :type "Float (single-precision)"))
  (`KismetSystemLibrary.PrintString` (`KismetStringLibrary.Conv_DoubleToString` (`/Game/DayNight/DayNightSystem/BP_DayNightSystem.GetHour` (`self.DayNight`))) true true (struct :`G` 0.66 :`B` 1.0 :`A` 1.0) 0.0)
  (`KismetSystemLibrary.PrintString` (`KismetSystemLibrary.GetDisplayName` (`self.CurrentAction`)) true true (struct :`G` 0.66 :`B` 1.0 :`A` 1.0) 0.0))

(event `self.ReceivePossess`
  (params (PossessedPawn :type "Pawn Object Reference"))
  (bind _returnvalue (`GameplayStatics.GetActorOfClass` "/Game/DayNight/DayNightSystem/BP_DayNightSystem.BP_DayNightSystem_C"))
  (bind _output_get (set `self.DayNight` _returnvalue))
  (`KismetSystemLibrary.K2_SetTimerDelegate` (`|CreateDelegate` :!event `CheckAction`) (`/Game/DayNight/DayNightSystem/BP_DayNightSystem.GetTimerRate` _output_get) true))

(event `CheckAction`
  (bind _action (`self.GetaAction`))
  (if (!= _action (`GameplayStatics.GetObjectClass` (`self.CurrentAction`)))
    (`self.CurrentAction`
      (:`then`
        (`/Game/AI/Blueprints/Actions/BP_action.Stop` (`self.CurrentAction`))
        (`KismetSystemLibrary.PrintString` "Hello4"))
      (:`else`
        _))
    (bind _returnvalue (`|SpawnActorFromClass` _action (`KismetMathLibrary.MakeTransform` (0.0 0.0 0.0)) "AlwaysSpawn" "OverrideRootScale" null (`self.K2_GetPawn`) null))
    (set `self.CurrentAction` _returnvalue)))

(fn `GetaAction`
  (returns (Action :type "/Game/AI/Blueprints/Actions/BP_action Class Reference"))
  (locals (L_Times :type "Array of Float (double-precision)") (L_Actions :type "Array of /Game/AI/Blueprints/Actions/BP_action Class Reference") (L_CurrentTime :type "Float (double-precision)" :default 0.0))
  (bind _l_times (`local.L_Times`))
  (bind _l_actions (`local.L_Actions`))
  (bind _schedule (message `/Game/AI/Blueprints/Interface/BPI_Schedule.GetSchedule` (`self.K2_GetPawn`)))
  (bind _keys (`BlueprintMapLibrary.Map_Keys` _schedule))
  (set `local.L_Times` _keys)
  (bind _values (`BlueprintMapLibrary.Map_Values` _schedule))
  (set `local.L_Actions` _values)
  (if (!= (`KismetArrayLibrary.Array_Length` (`local.L_Times`)) 0)
    (set `local.L_CurrentTime` (`/Game/DayNight/DayNightSystem/BP_DayNightSystem.GetHour` (`self.DayNight`)))
    (if (or (< (`local.L_CurrentTime`) (`|GetArrayItem` (`local.L_Times`))) (>= (`local.L_CurrentTime`) (`|GetArrayItem` _l_times (`KismetArrayLibrary.Array_LastIndex` _l_times))))
      (return (`|GetArrayItem` _l_actions (`KismetArrayLibrary.Array_LastIndex` _l_actions)))
      (else
        (for (_array_element _array_index) (`local.L_Times`)
          (if (and (>= (`local.L_CurrentTime`) _array_element) (< (`local.L_CurrentTime`) (`|GetArrayItem` (`local.L_Times`) (+ _array_index 1))))
            (return (`|GetArrayItem` (`local.L_Actions`) _array_index))))
        (return null)))
    (else
      (return null))))

(fn `UserConstructionScript`)