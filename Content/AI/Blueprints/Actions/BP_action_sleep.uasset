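; AI action Blueprint that sends a pawn to its bed to sleep.
; Task gets the bed through a pawn message and, if valid, uses AIMoveTo to reach its location.
; On arrival it sets the pawn's yaw from a look-at between its own location and itself, not the bed, then starts sleeping.
; Stop sends the stop-sleeping message before calling the parent Stop.
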(event `self.Task`
  (bind _pawn (`self.Pawn`))
  (bind (_returnvalue_roll _returnvalue_pitch _returnvalue_yaw) (`KismetMathLibrary.BreakRotator` (`KismetMathLibrary.FindLookAtRotation` (`self.K2_GetActorLocation` _pawn) (`self.K2_GetActorLocation` _pawn))))
  (`parent.Task`)
  (bind (_bed _placebed) (message `/Game/AI/Blueprints/Interface/BPBI_sleep.GetBed` (`self.Pawn`)))
  (`/Engine/EditorBlueprintResources/StandardMacros.IsValid` _placebed
    (:`Is Valid`
      (`|AIMoveTo` (`self.Pawn`) (`/Game/AI/Blueprints/Places/BP_Place.GetLocation` _placebed) null (`self.Acceptance Radius`)
        (:`OnSuccess`
          (`self.K2_SetActorRotation` (`self.Pawn`) (`KismetMathLibrary.MakeRotator` 0.0 0.0 _returnvalue_yaw) false)
          (message `/Game/AI/Blueprints/Interface/BPBI_sleep.StartSleeping` (`self.Pawn`)))))))

(event `self.Stop`
  (message `/Game/AI/Blueprints/Interface/BPBI_sleep.StopSleeping` (`self.Pawn`))
  (`parent.Stop`))

(fn `UserConstructionScript`
  (`parent.UserConstructionScript`))