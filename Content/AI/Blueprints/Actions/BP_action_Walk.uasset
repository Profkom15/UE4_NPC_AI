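; AI action Blueprint that keeps its pawn walking from point to point in an endless loop.
; Its Task event calls the parent task, asks the pawn for a destination through an interface message, and issues an AI MoveTo using the action's acceptance radius.
; Success and failure both wait for a delay supplied by the pawn, then call Task again to pick the next location.
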(event `self.Task`
  (`parent.Task`)
  (bind _location (message `/Game/AI/Blueprints/Interface/BPI_Walk.GetWalkLocation` (`self.Pawn`)))
  (`|AIMoveTo` (`self.Pawn`) _location null (`self.Acceptance Radius`)
    (:`OnSuccess`
      _)
    (:`OnFail`
      _))
  (bind _delay (message `/Game/AI/Blueprints/Interface/BPI_Walk.GetWalkDelay` (`self.Pawn`)))
  (`KismetSystemLibrary.Delay` _delay)
  (`self.Task`))

(fn `UserConstructionScript`
  (`parent.UserConstructionScript`))